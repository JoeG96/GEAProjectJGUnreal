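; CCTV monitor Blueprint with one big and three small screens, accepting player key input only while its overlap box is overlapped.
; Divide flip-flops the big screen between on and a blank floor material; when on, Space cycles three render-target materials through a looping MultiGate.
; Multiply loops over the second found CCTVBP's TextureArray, setting every element on all three small screens, so the last one remains.
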(event OnComponentBeginOverlap(OverlapBox)
  (params (OverlappedComponent :type Primitive%20Component%20Object%20Reference) (OtherActor :type Actor%20Object%20Reference) (OtherComp :type Primitive%20Component%20Object%20Reference) (OtherBodyIndex :type Integer) (bFromSweep :type Boolean) (SweepResult :type Hit%20Result%20Structure%20%28by%20ref%29))
  ;[1 1 1] Input enabled/disabled with overlap
  (Input|EnableInput (Game|GetPlayerController 0)))

(event OnComponentEndOverlap(OverlapBox)
  (params (OverlappedComponent :type Primitive%20Component%20Object%20Reference) (OtherActor :type Actor%20Object%20Reference) (OtherComp :type Primitive%20Component%20Object%20Reference) (OtherBodyIndex :type Integer))
  ;[1 1 1] Input enabled/disabled with overlap
  (Input|DisableInput 0))

(event EventBeginPlay)

(event Collision|EventActorBeginOverlap
  (params (OtherActor :type Actor%20Object%20Reference)))

(event EventTick
  (params (DeltaSeconds :type Float%20%28single-precision%29)))

(event Input|KeyboardEvents|Subtract
  (params (Key :type Key%20Structure :default "None"))
  (:Pressed
    (if (Variables|Default|Getdisplay_on)
      _)))

(event Input|KeyboardEvents|SpaceBar
  (params (Key :type Key%20Structure :default "None"))
  (bind _cctvscreenbig (Variables|Default|GetCCTVScreenBig))
  ;[1 1 1] Input enabled when overlapping, use key to turn off on, space to cycle through textures (Single Display)
  (:Pressed
    (if (Variables|Default|Getdisplay_on)
      (Utilities|FlowControl|MultiGate false true -1
        (:Out%200
          (Rendering|Material|SetMaterial _cctvscreenbig 0 "/Game/CCTV/CCTVRenderTarget1_Mat.CCTVRenderTarget1_Mat"))
        (:Out%201
          (Rendering|Material|SetMaterial _cctvscreenbig 0 "/Game/CCTV/CCTVRenderTarget2_Mat.CCTVRenderTarget2_Mat"))
        (:Out%202
          (Rendering|Material|SetMaterial _cctvscreenbig 0 "/Game/CCTV/CCTVRenderTarget3_Mat.CCTVRenderTarget3_Mat"))))))

(event Input|KeyboardEvents|Divide
  (params (Key :type Key%20Structure :default "None"))
  (bind _cctvscreenbig (Variables|Default|GetCCTVScreenBig))
  ;[1 1 1] Input enabled when overlapping, use key to turn off on, space to cycle through textures (Single Display)
  (:Pressed
    (Utilities|FlowControl|FlipFlop
      (:A
        (Variables|Default|Setdisplay_on true)
        (if (Variables|Default|Getdisplay_on)
          (Utilities|FlowControl|MultiGate false true -1
            (:Out%200
              (Rendering|Material|SetMaterial _cctvscreenbig 0 "/Game/CCTV/CCTVRenderTarget1_Mat.CCTVRenderTarget1_Mat"))
            (:Out%201
              (Rendering|Material|SetMaterial _cctvscreenbig 0 "/Game/CCTV/CCTVRenderTarget2_Mat.CCTVRenderTarget2_Mat"))
            (:Out%202
              (Rendering|Material|SetMaterial _cctvscreenbig 0 "/Game/CCTV/CCTVRenderTarget3_Mat.CCTVRenderTarget3_Mat")))))
      (:B
        (Variables|Default|Setdisplay_on false)
        (Rendering|Material|SetMaterial _cctvscreenbig 0 "/Engine/EditorMaterials/Thumbnails/FloorPlaneMaterial.FloorPlaneMaterial")))))

(event Input|KeyboardEvents|Multiply
  (params (Key :type Key%20Structure :default "None"))
  (:Pressed
    (bind _outactors (Actor|GetAllActorsOfClass "CCTVBP_C"))
    (for _array_element (Variables|CCTVBP_C|Gettexture_array (Utilities|Array|Get(acopy) _outactors 1))
      (Rendering|Material|SetMaterial (Variables|Default|GetCCTVScreenSmall3) 0 _array_element))))

(fn ConstructionScript)