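; Projector actor that plays a short film through a media player and controls three colored spotlights, taking key input only while something overlaps its interaction box.
; Q and E play and reverse a timeline that scales the intensity of the red, green and blue child-actor lights.
; Other keys toggle pause, set fast reverse or forward playback, and close or reopen the film, seeking back to the saved time when it reopens.
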(event OnComponentEndOverlap(InteractionBox)
  (params (OverlappedComponent :type Primitive%20Component%20Object%20Reference) (OtherActor :type Actor%20Object%20Reference) (OtherComp :type Primitive%20Component%20Object%20Reference) (OtherBodyIndex :type Integer))
  (Input|DisableInput (Game|GetPlayerController 0)))

(event OnComponentBeginOverlap(InteractionBox)
  (params (OverlappedComponent :type Primitive%20Component%20Object%20Reference) (OtherActor :type Actor%20Object%20Reference) (OtherComp :type Primitive%20Component%20Object%20Reference) (OtherBodyIndex :type Integer) (bFromSweep :type Boolean) (SweepResult :type Hit%20Result%20Structure%20%28by%20ref%29))
  (Input|EnableInput (Game|GetPlayerController 0)))

(event Custom|OnMediaOpened_Event_0
  (params (OpenedUrl :type String))
  (bind _mediaplayer (Variables|Default|GetMediaPlayer))
  ;[1 1 1] Close player with button press and resume with same press
  (Media|MediaPlayer|Seek _mediaplayer (Variables|Default|GetStopTime))
  (Media|MediaPlayer|Play _mediaplayer :!class /Script/MediaAssets.MediaPlayer))

(event EventBeginPlay
  (Media|MediaPlayer|OpenSource (Variables|Default|GetMediaPlayer) "/Game/Movies/Save_Ralph_-_A_short_film_with_Taika_Waititi.Save_Ralph_-_A_short_film_with_Taika_Waititi"))

(event EventTick
  (params (DeltaSeconds :type Float%20%28single-precision%29)))

(event Input|KeyboardEvents|P
  (params (Key :type Key%20Structure :default "None"))
  (bind _mediaplayer (Variables|Default|GetMediaPlayer))
  ;[1 1 1] Pause/Play media player
  (:Pressed
    (Utilities|FlowControl|FlipFlop
      (:A
        (Media|MediaPlayer|Play _mediaplayer :!class /Script/MediaAssets.MediaPlayer))
      (:B
        (Sequencer|Player|Pause _mediaplayer)))))

(event Input|KeyboardEvents|LeftBracket
  (params (Key :type Key%20Structure :default "None"))
  ;[1 1 1] Change playback to reverse/forward
  (:Pressed
    (Class|MediaPlayer|SetRate (Variables|Default|GetMediaPlayer) -2.0)))

(event Input|KeyboardEvents|RightBracket
  (params (Key :type Key%20Structure :default "None"))
  ;[1 1 1] Change playback to reverse/forward
  (:Pressed
    (Class|MediaPlayer|SetRate (Variables|Default|GetMediaPlayer) 2.0)))

(event Input|KeyboardEvents|Down
  (params (Key :type Key%20Structure :default "None"))
  (bind _mediaplayer (Variables|Default|GetMediaPlayer))
  ;[1 1 1] Close player with button press and resume with same press
  (:Pressed
    (Utilities|FlowControl|FlipFlop
      (:A
        (Variables|Default|SetStopTime (Class|MediaPlayer|GetTime _mediaplayer))
        (Media|MediaPlayer|Close _mediaplayer :!class /Script/MediaAssets.MediaPlayer))
      (:B
        (Media|MediaPlayer|OpenSource _mediaplayer "/Game/Movies/Save_Ralph_-_A_short_film_with_Taika_Waititi.Save_Ralph_-_A_short_film_with_Taika_Waititi")
        (Media|MediaPlayer|BindEventtoOnMediaOpened _mediaplayer (delegate Custom|OnMediaOpened_Event_0))))))

(event Input|KeyboardEvents|E
  (params (Key :type Key%20Structure :default "None"))
  ;[1 1 1] Casts child actor to light, uses timeline to increase intensity when overlap with detection cube or chosen keys
  (:Released
    (bind _lightbrightnessfloattrack (Timeline|FadeInTimeline Reverse)
      (:Update
        (Utilities|FlowControl|Sequence
          (:then_0
            (bind _aslight (Utilities|Casting|CastToLight (Variables|/Script/Engine.ChildActorComponent|GetChildActor (Variables|Default|GetSpotLightBlue))))
            (Rendering|Components|Light|SetIntensity (Variables|/Script/Engine.Light|GetLightComponent _aslight) (* _lightbrightnessfloattrack (Variables|Default|GetBrightnessMultiplier))))
          (:then_1
            (bind _aslight_2 (Utilities|Casting|CastToLight (Variables|/Script/Engine.ChildActorComponent|GetChildActor (Variables|Default|GetSpotLightGreen))))
            (Rendering|Components|Light|SetIntensity (Variables|/Script/Engine.Light|GetLightComponent _aslight_2) (* _lightbrightnessfloattrack (Variables|Default|GetBrightnessMultiplier))))
          (:then_2
            (bind _aslight_3 (Utilities|Casting|CastToLight (Variables|/Script/Engine.ChildActorComponent|GetChildActor (Variables|Default|GetSpotLightRed))))
            (Rendering|Components|Light|SetIntensity (Variables|/Script/Engine.Light|GetLightComponent _aslight_3) (* _lightbrightnessfloattrack (Variables|Default|GetBrightnessMultiplier)))))))))

(event Input|KeyboardEvents|Q
  (params (Key :type Key%20Structure :default "None"))
  ;[1 1 1] Casts child actor to light, uses timeline to increase intensity when overlap with detection cube or chosen keys
  (:Released
    (bind _lightbrightnessfloattrack (Timeline|FadeInTimeline Play)
      (:Update
        (Utilities|FlowControl|Sequence
          (:then_0
            (bind _aslight (Utilities|Casting|CastToLight (Variables|/Script/Engine.ChildActorComponent|GetChildActor (Variables|Default|GetSpotLightBlue))))
            (Rendering|Components|Light|SetIntensity (Variables|/Script/Engine.Light|GetLightComponent _aslight) (* _lightbrightnessfloattrack (Variables|Default|GetBrightnessMultiplier))))
          (:then_1
            (bind _aslight_2 (Utilities|Casting|CastToLight (Variables|/Script/Engine.ChildActorComponent|GetChildActor (Variables|Default|GetSpotLightGreen))))
            (Rendering|Components|Light|SetIntensity (Variables|/Script/Engine.Light|GetLightComponent _aslight_2) (* _lightbrightnessfloattrack (Variables|Default|GetBrightnessMultiplier))))
          (:then_2
            (bind _aslight_3 (Utilities|Casting|CastToLight (Variables|/Script/Engine.ChildActorComponent|GetChildActor (Variables|Default|GetSpotLightRed))))
            (Rendering|Components|Light|SetIntensity (Variables|/Script/Engine.Light|GetLightComponent _aslight_3) (* _lightbrightnessfloattrack (Variables|Default|GetBrightnessMultiplier)))))))))

(fn ConstructionScript)