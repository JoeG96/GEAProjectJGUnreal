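; Projector actor that casts red, green and blue spotlights and controls media playback, taking key input only while something overlaps its InteractionBox.
; A timeline fades the three child-actor lights in and out, driving intensity and applying each one's light function material.
; Keys open, pause, close and resume the first media source at its saved time, or set fast forward and reverse rates.
; Another key stores a random image material in MasterInstanceMaterial.
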(event OnComponentEndOverlap(InteractionBox)
  (params (OverlappedComponent :type Primitive%20Component%20Object%20Reference) (OtherActor :type Actor%20Object%20Reference) (OtherComp :type Primitive%20Component%20Object%20Reference) (OtherBodyIndex :type Integer))
  (Input|DisableInput (Game|GetPlayerController 0)))

(event OnComponentBeginOverlap(InteractionBox)
  (params (OverlappedComponent :type Primitive%20Component%20Object%20Reference) (OtherActor :type Actor%20Object%20Reference) (OtherComp :type Primitive%20Component%20Object%20Reference) (OtherBodyIndex :type Integer) (bFromSweep :type Boolean) (SweepResult :type Hit%20Result%20Structure%20%28by%20ref%29))
  (Input|EnableInput (Game|GetPlayerController 0)))

(event Custom|OnMediaOpened_Event_0
  (params (OpenedUrl :type String))
  (bind _mediaplayer (Variables|Default|GetMediaPlayer))
  ;[1 1 1] Close player with button press and resume with same press
  (Media|MediaPlayer|Seek _mediaplayer (Variables|Default|GetStopTime))
  (Media|MediaPlayer|Play _mediaplayer :!class /Script/MediaAssets.MediaPlayer))

(event EventBeginPlay)

(event EventEndPlay
  (params (EndPlayReason :type EEndPlayReason%20Enum :default "Destroyed"))
  (Media|MediaPlayer|Close (Variables|Default|GetMediaPlayer) :!class /Script/MediaAssets.MediaPlayer))

(event EventTick
  (params (DeltaSeconds :type Float%20%28single-precision%29)))

(event Input|KeyboardEvents|P
  (params (Key :type Key%20Structure :default "None"))
  (bind _mediaplayer (Variables|Default|GetMediaPlayer))
  ;[1 1 1] Pause/Play media player
  (:Pressed
    (Utilities|FlowControl|FlipFlop
      (:A
        (Media|MediaPlayer|Play _mediaplayer :!class /Script/MediaAssets.MediaPlayer))
      (:B
        (Sequencer|Player|Pause _mediaplayer)))))

(event Input|KeyboardEvents|LeftBracket
  (params (Key :type Key%20Structure :default "None"))
  ;[1 1 1] Change playback to reverse/forward
  (:Pressed
    (Class|MediaPlayer|SetRate (Variables|Default|GetMediaPlayer) -2.0)))

(event Input|KeyboardEvents|RightBracket
  (params (Key :type Key%20Structure :default "None"))
  ;[1 1 1] Change playback to reverse/forward
  (:Pressed
    (Class|MediaPlayer|SetRate (Variables|Default|GetMediaPlayer) 2.0)))

(event Input|KeyboardEvents|Down
  (params (Key :type Key%20Structure :default "None"))
  (bind _mediaplayer (Variables|Default|GetMediaPlayer))
  ;[1 1 1] Close player with button press and resume with same press
  (:Pressed
    (Utilities|FlowControl|FlipFlop
      (:A
        (Variables|Default|SetStopTime (Class|MediaPlayer|GetTime _mediaplayer))
        (Media|MediaPlayer|Close _mediaplayer :!class /Script/MediaAssets.MediaPlayer))
      (:B
        (Media|MediaPlayer|OpenSource _mediaplayer (Utilities|Array|Get(acopy) (Variables|Default|GetMediaArray)))
        (Media|MediaPlayer|BindEventtoOnMediaOpened _mediaplayer (delegate Custom|OnMediaOpened_Event_0))))))

(event Input|KeyboardEvents|L
  (params (Key :type Key%20Structure :default "None"))
  (:Pressed
    (Media|MediaPlayer|OpenSource (Variables|Default|GetMediaPlayer) (Utilities|Array|Get(acopy) (Variables|Default|GetMediaArray)))))

(event Input|KeyboardEvents|E
  (params (Key :type Key%20Structure :default "None"))
  ;[1 1 1] Casts child actor to light, uses timeline to increase intensity when overlap with detection cube or chosen keys
  (:Released
    (bind _lightbrightnessfloattrack (Timeline|FadeInTimeline Reverse)
      (:Update
        (Utilities|FlowControl|Sequence
          (:then_0
            (bind _aslight (Utilities|Casting|CastToLight (Variables|/Script/Engine.ChildActorComponent|GetChildActor (Variables|Components|GetSpotLightBlue))))
            (Rendering|Components|Light|SetIntensity (Variables|/Script/Engine.Light|GetLightComponent _aslight) (* _lightbrightnessfloattrack (Variables|Default|GetBrightnessMultiplier)))
            (Rendering|Components|Light|SetLightFunctionMaterial (Variables|/Script/Engine.Light|GetLightComponent _aslight) (Variables|Default|GetSpotlightMatBlue)))
          (:then_1
            (bind _aslight_2 (Utilities|Casting|CastToLight (Variables|/Script/Engine.ChildActorComponent|GetChildActor (Variables|Components|GetSpotLightGreen))))
            (Rendering|Components|Light|SetIntensity (Variables|/Script/Engine.Light|GetLightComponent _aslight_2) (* _lightbrightnessfloattrack (Variables|Default|GetBrightnessMultiplier)))
            (Rendering|Components|Light|SetLightFunctionMaterial (Variables|/Script/Engine.Light|GetLightComponent _aslight_2) (Variables|Default|GetSpotlightMatGreen)))
          (:then_2
            (bind _aslight_3 (Utilities|Casting|CastToLight (Variables|/Script/Engine.ChildActorComponent|GetChildActor (Variables|Components|GetSpotLightRed))))
            (Rendering|Components|Light|SetIntensity (Variables|/Script/Engine.Light|GetLightComponent _aslight_3) (* _lightbrightnessfloattrack (Variables|Default|GetBrightnessMultiplier)))
            (Rendering|Components|Light|SetLightFunctionMaterial (Variables|/Script/Engine.Light|GetLightComponent _aslight_3) (Variables|Default|GetSpotlightMatRed))))))))

(event Input|KeyboardEvents|Q
  (params (Key :type Key%20Structure :default "None"))
  ;[1 1 1] Casts child actor to light, uses timeline to increase intensity when overlap with detection cube or chosen keys
  (:Released
    (bind _lightbrightnessfloattrack (Timeline|FadeInTimeline Play)
      (:Update
        (Utilities|FlowControl|Sequence
          (:then_0
            (bind _aslight (Utilities|Casting|CastToLight (Variables|/Script/Engine.ChildActorComponent|GetChildActor (Variables|Components|GetSpotLightBlue))))
            (Rendering|Components|Light|SetIntensity (Variables|/Script/Engine.Light|GetLightComponent _aslight) (* _lightbrightnessfloattrack (Variables|Default|GetBrightnessMultiplier)))
            (Rendering|Components|Light|SetLightFunctionMaterial (Variables|/Script/Engine.Light|GetLightComponent _aslight) (Variables|Default|GetSpotlightMatBlue)))
          (:then_1
            (bind _aslight_2 (Utilities|Casting|CastToLight (Variables|/Script/Engine.ChildActorComponent|GetChildActor (Variables|Components|GetSpotLightGreen))))
            (Rendering|Components|Light|SetIntensity (Variables|/Script/Engine.Light|GetLightComponent _aslight_2) (* _lightbrightnessfloattrack (Variables|Default|GetBrightnessMultiplier)))
            (Rendering|Components|Light|SetLightFunctionMaterial (Variables|/Script/Engine.Light|GetLightComponent _aslight_2) (Variables|Default|GetSpotlightMatGreen)))
          (:then_2
            (bind _aslight_3 (Utilities|Casting|CastToLight (Variables|/Script/Engine.ChildActorComponent|GetChildActor (Variables|Components|GetSpotLightRed))))
            (Rendering|Components|Light|SetIntensity (Variables|/Script/Engine.Light|GetLightComponent _aslight_3) (* _lightbrightnessfloattrack (Variables|Default|GetBrightnessMultiplier)))
            (Rendering|Components|Light|SetLightFunctionMaterial (Variables|/Script/Engine.Light|GetLightComponent _aslight_3) (Variables|Default|GetSpotlightMatRed))))))))

(event Input|KeyboardEvents|C
  (params (Key :type Key%20Structure :default "None"))
  (bind _imagearray (Variables|Default|GetImageArray))
  (:Pressed
    (Variables|Default|SetMasterInstanceMaterial (Utilities|Array|Get(acopy) _imagearray (Math|Random|RandomInteger (+ (Utilities|Array|LastIndex _imagearray) 1))))))

(fn ConstructionScript)